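; DynamicMaterialsController creates dynamic material instances for mesh slots and drives their color and blend parameters.
; SetupMaterial picks a source material from a list by ID, creates the instance, stores it by slot index and sets its base color.
; Setters look up that slot to update base color, fuzz color or wall blending: corner positions, four-sided mask ranges and inner/outer mask colors.
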(fn `SetBaseColor`
  (params (MaterialID :type Integer) (Color :type "LinearColor Structure"))
  (bind (_value _returnvalue) (`BlueprintMapLibrary.Map_Find` (`self.Materials`) MaterialID))
  (if _returnvalue
    (`MaterialInstanceDynamic.SetVectorParameterValue` _value "BaseColor" Color)))

(fn `SetFuzzColor`
  (params (MeshMaterialID :type Integer) (Color :type "LinearColor Structure"))
  (bind (_value _returnvalue) (`BlueprintMapLibrary.Map_Find` (`self.Materials`) MeshMaterialID))
  (if _returnvalue
    (`MaterialInstanceDynamic.SetVectorParameterValue` _value "FuzzColor" Color)))

(fn `SetMaterialBlendValues`
  (params (MeshMaterialID :type "Integer (by ref)") (WallMaterial :type "/Game/Blueprints/Walls/Lists/WallMaterial Structure (by ref)") (InnerColor :type "LinearColor Structure") (OuterColor :type "LinearColor Structure") (BottomLeft :type "Vector Structure") (TopRight :type "Vector Structure"))
  (bind (_leftmask _leftmaskrange _rightmask _rightmaskrange _bottommask _bottommaskrange _topmask _topmaskrange) (break `/Game/Blueprints/Walls/Lists/WallMaterial` WallMaterial))
  (bind (_value _returnvalue) (`BlueprintMapLibrary.Map_Find` (`self.Materials`) MeshMaterialID))
  (if _returnvalue
    (`|ExecutionSequence`
      (:`then_0`
        (`MaterialInstanceDynamic.SetVectorParameterValue` _value "BlendPositionBottomLeft" (`KismetMathLibrary.Conv_VectorToLinearColor` BottomLeft))
        (`MaterialInstanceDynamic.SetVectorParameterValue` _value "BlendPositionTopRight" (`KismetMathLibrary.Conv_VectorToLinearColor` TopRight))
        (`MaterialInstanceDynamic.SetScalarParameterValue` _value "LeftMin" _leftmask)
        (`MaterialInstanceDynamic.SetScalarParameterValue` _value "LeftRange" _leftmaskrange)
        (`MaterialInstanceDynamic.SetScalarParameterValue` _value "RightMin" _rightmask)
        (`MaterialInstanceDynamic.SetScalarParameterValue` _value "RightRange" _rightmaskrange)
        (`MaterialInstanceDynamic.SetScalarParameterValue` _value "BottomMin" _bottommask)
        (`MaterialInstanceDynamic.SetScalarParameterValue` _value "BottomRange" _bottommaskrange)
        (`MaterialInstanceDynamic.SetScalarParameterValue` _value "TopMin" _topmask)
        (`MaterialInstanceDynamic.SetScalarParameterValue` _value "TopRange" _topmaskrange))
      (:`then_1`
        (`MaterialInstanceDynamic.SetVectorParameterValue` _value "InnerMaskColor" InnerColor)
        (`MaterialInstanceDynamic.SetVectorParameterValue` _value "CombinedMaskColor" OuterColor)))))

(fn `SetupMaterial`
  (params (Materials :type "Array of MaterialInstance Object Reference") (MaterialID :type Integer) (Mesh :type "PrimitiveComponent Object Reference") (MeshMaterialID :type Integer) (Color :type "LinearColor Structure"))
  (bind (_hasitems _selectedmaterial) (`/Game/Blueprints/Controller/AssetsFunctionLibrary.GetSourceMaterial` Materials MaterialID))
  (if _hasitems
    (bind _returnvalue (`PrimitiveComponent.CreateDynamicMaterialInstance` Mesh MeshMaterialID _selectedmaterial))
    (`BlueprintMapLibrary.Map_Add` (`self.Materials`) MeshMaterialID _returnvalue)
    (`self.SetBaseColor` MeshMaterialID Color)))