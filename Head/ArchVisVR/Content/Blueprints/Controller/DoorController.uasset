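; Door controller component on a DoorBase actor that runs opening, closing, self-closing and lock states.
; Interaction starts opening or closing, or unlocks a locked door, and enables component tick only while needed.
; Once the grip is flagged as handled, tick rotates door and grip from DoorBase's vector curves, mirroring yaw for left doors.
; Self-closing doors keep ticking while open and close when the player moves beyond a set distance.
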(event `self.ReceiveBeginPlay`
  (bind _asdoor_base (cast `/Game/Blueprints/Doors/DoorBase` (`self.GetOwner`)))
  (set `self.DoorGrip` (`/Game/Blueprints/Doors/DoorBase.DoorGrip` _asdoor_base))
  (set `self.Door` (`/Game/Blueprints/Doors/DoorBase.Door` _asdoor_base))
  (set `self.DoorOpenAnimCurve` (`/Game/Blueprints/Doors/DoorBase.DoorOpenAnimCurve` _asdoor_base))
  (set `self.DoorCloseAnimCuve` (`/Game/Blueprints/Doors/DoorBase.DoorCloseAnimCuve` _asdoor_base)))

(event `self.ReceiveTick`
  (params (DeltaSeconds :type "Float (single-precision)"))
  (`self.HandleDoor` DeltaSeconds))

(event `InteractWithDoor`
  (if (not (`self.IsComponentTickEnabled`))
    (switch `/Game/Blueprints/Doors/DoorStates` (`self.DoorStates`)
      (:`NewEnumerator1`
        (set `self.IsClosing` true)
        (set `self.IsGripHandled` true)
        (set `self.DoorStates` "NewEnumerator2")
        (`self.SetComponentTickEnabled` true))
      (:`NewEnumerator4`
        (set `self.DoorGripState` "NewEnumerator1")
        (set `self.DoorStates` "NewEnumerator0")
        (`self.SetComponentTickEnabled` true))
      (:`NewEnumerator3`
        (`self.LockDoor`)))))

(fn `DistanceToPlayer`
  (returns (DistanceCheck :type Boolean))
  (return (>= (`KismetMathLibrary.VSize` (- (`Actor.K2_GetActorLocation` (`GameplayStatics.GetPlayerPawn` 0)) (`Actor.K2_GetActorLocation` (`self.GetOwner`)))) (`self.PlayMaxDistance`))))

(fn `HandleDoor`
  (params (DeltaSeconds :type "Float (double-precision)"))
  (bind _distancecheck (`self.DistanceToPlayer`))
  (bind _returnvalue (select `/Game/Blueprints/Doors/DoorStates` (`self.DoorStates`) :`NewEnumerator0` (.x (`self.DoorOpenTime`)) :`NewEnumerator1` 1.0 :`NewEnumerator2` (.y (`self.DoorOpenTime`)) :`NewEnumerator4` 1.0 :`NewEnumerator3` 1.0))
  (if (`self.IsGripHandled`)
    (bind _output_get (set `self.DoorOpen` (+ (`self.DoorOpen`) (/ DeltaSeconds _returnvalue))))
    (switch `/Game/Blueprints/Doors/DoorStates` (`self.DoorStates`)
      (:`NewEnumerator0`
        (bind _z (.z (`CurveVector.GetVectorValue` (`self.DoorOpenAnimCurve`) (`KismetMathLibrary.FClamp` _output_get))))
        (`SceneComponent.K2_SetRelativeRotation` (`self.Door`) (`KismetMathLibrary.MakeRotator` (.x (`CurveVector.GetVectorValue` (`self.DoorOpenAnimCurve`) (`KismetMathLibrary.FClamp` _output_get))) (.y (`CurveVector.GetVectorValue` (`self.DoorOpenAnimCurve`) (`KismetMathLibrary.FClamp` _output_get))) (`KismetMathLibrary.SelectFloat` (* _z -1.0) _z (`self.IsLeft`))) false false)
        (`SceneComponent.K2_SetRelativeRotation` (`self.DoorGrip`) (`KismetMathLibrary.MakeRotator` (.x (`CurveVector.GetVectorValue` (`self.DoorOpenAnimCurve`) (`KismetMathLibrary.FClamp` _output_get))) (.y (`CurveVector.GetVectorValue` (`self.DoorOpenAnimCurve`) (`KismetMathLibrary.FClamp` _output_get))) (`KismetMathLibrary.SelectFloat` (* _z -1.0) _z (`self.IsLeft`))) false false))
      (:`NewEnumerator1`
        _)
      (:`NewEnumerator2`
        (bind _returnvalue_2 (`KismetMathLibrary.FClamp` _output_get))
        (bind _z_2 (.z (`CurveVector.GetVectorValue` (`self.DoorCloseAnimCuve`) _returnvalue_2)))
        (`SceneComponent.K2_SetRelativeRotation` (`self.Door`) (`KismetMathLibrary.MakeRotator` (.x (`CurveVector.GetVectorValue` (`self.DoorCloseAnimCuve`) _returnvalue_2)) (.y (`CurveVector.GetVectorValue` (`self.DoorCloseAnimCuve`) _returnvalue_2)) (`KismetMathLibrary.SelectFloat` (* _z_2 -1.0) _z_2 (`self.IsLeft`))) false false)
        (`SceneComponent.K2_SetRelativeRotation` (`self.DoorGrip`) (`KismetMathLibrary.MakeRotator` (.x (`CurveVector.GetVectorValue` (`self.DoorCloseAnimCuve`) _returnvalue_2)) (.y (`CurveVector.GetVectorValue` (`self.DoorCloseAnimCuve`) _returnvalue_2)) (`KismetMathLibrary.SelectFloat` (* _z_2 -1.0) _z_2 (`self.IsLeft`))) false false)
        (if (and (>= _returnvalue_2 0.9) (`self.IsClosing`))
          (set `self.DoorGripState` "NewEnumerator1")
          (set `self.IsClosing` false))))
    (bind _returnvalue_3 (>= _output_get _returnvalue))
    (if (select `/Game/Blueprints/Doors/DoorStates` (`self.DoorStates`) :`NewEnumerator0` _returnvalue_3 :`NewEnumerator1` _distancecheck :`NewEnumerator2` _returnvalue_3 :`NewEnumerator4` _distancecheck :`NewEnumerator3` _distancecheck)
      (bind _output_get_2 (set `self.DoorStates` (select `/Game/Blueprints/Doors/DoorStates` (`self.DoorStates`) :`NewEnumerator0` "NewEnumerator1" :`NewEnumerator1` "NewEnumerator2" :`NewEnumerator2` "NewEnumerator4" :`NewEnumerator4` "NewEnumerator4" :`NewEnumerator3` "NewEnumerator3" :!type "/Game/Blueprints/Doors/DoorStates Enum")))
      (set `self.DoorOpen` 0.0)
      (set `self.IsClosing` (`|EnumEquality` _output_get_2 "NewEnumerator2"))
      (if (or (not (`self.IsSelfClosing`)) (`|EnumEquality` _output_get_2 "NewEnumerator4") (`|EnumEquality` _output_get_2 "NewEnumerator3"))
        (`self.SetComponentTickEnabled` false)))))

(fn `LockDoor`
  (set `self.DoorStates` (select `/Game/Blueprints/Doors/DoorStates` (`self.DoorStates`) :`NewEnumerator0` "NewEnumerator3" :`NewEnumerator1` "NewEnumerator3" :`NewEnumerator2` "NewEnumerator3" :`NewEnumerator4` "NewEnumerator3" :`NewEnumerator3` "NewEnumerator4" :!type "/Game/Blueprints/Doors/DoorStates Enum")))