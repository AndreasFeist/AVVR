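; Blueprint function library that looks up meshes, materials and door frames for modular building walls.
; List getters return the item at an ID, fall back to index 0 when it exceeds the last index, and report whether the list has items.
; GetWallMesh picks the mesh for a wall type from a map keyed by wall height.
; SocketTypeToID collapses wall, balcony, cellar window, door and window variants into shared integer IDs.
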(fn `GetDoorStruct`
  (params (FramesList :type "Array of /Game/Blueprints/Doors/Lists/DoorSStruct Structure") (DoorFrameID :type Integer))
  (returns (HasItems :type Boolean) (Frame :type "/Game/Blueprints/Doors/Lists/DoorSStruct Structure"))
  (bind _returnvalue (> (`KismetArrayLibrary.Array_Length` FramesList) 0))
  (if _returnvalue
    (return _returnvalue (`|GetArrayItem` FramesList (`KismetMathLibrary.SelectInt` DoorFrameID 0 (<= DoorFrameID (`KismetArrayLibrary.Array_LastIndex` FramesList)))))
    (else
      (return _returnvalue))))

(fn `GetSourceMaterial`
  (params (MaterialsList :type "Array of MaterialInstance Object Reference (by ref)") (CurrentID :type Integer))
  (returns (HasItems :type Boolean) (SelectedMaterial :type "MaterialInstance Object Reference"))
  (bind _returnvalue (> (`KismetArrayLibrary.Array_Length` MaterialsList) 0))
  (if _returnvalue
    (return _returnvalue (`|GetArrayItem` MaterialsList (`KismetMathLibrary.SelectInt` CurrentID 0 (<= CurrentID (`KismetArrayLibrary.Array_LastIndex` MaterialsList)))))
    (else
      (return _returnvalue null))))

(fn `GetStaticMesh`
  (params (AssetList :type "Array of StaticMesh Object Reference (by ref)") (CurrentID :type Integer))
  (returns (HasItems :type Boolean) (Mesh :type "StaticMesh Object Reference") (ID :type Integer))
  (bind _returnvalue (> (`KismetArrayLibrary.Array_Length` AssetList) 0))
  (bind _returnvalue_2 (`KismetMathLibrary.SelectInt` CurrentID 0 (<= CurrentID (`KismetArrayLibrary.Array_LastIndex` AssetList))))
  (if _returnvalue
    (return _returnvalue (`|GetArrayItem` AssetList _returnvalue_2) _returnvalue_2)
    (else
      (return _returnvalue null 0))))

(fn `GetWallMesh`
  (params (WallType :type "/Game/Blueprints/Walls/Lists/WallTypes Enum" :default "NewEnumerator8") (WallMeshesMap :type "Map of /Game/Blueprints/Walls/Lists/WallHeight Enum to /Game/Blueprints/Walls/Lists/WallMeshesStruct Structure (by ref)" :default _) (WallHeight :type "/Game/Blueprints/Walls/Lists/WallHeight Enum" :default "NewEnumerator5"))
  (returns (Mesh :type "StaticMesh Object Reference"))
  (bind (_value _returnvalue) (`BlueprintMapLibrary.Map_Find` WallMeshesMap WallHeight))
  (bind (_wallmesh _wall_narrow01mesh _wall_narrow02mesh _wall_narrow03mesh _wall_narrow04mesh _wall_smallmesh _balconymesh _balcony_leftmesh _balcony_centermesh _balcony_rightmesh _cellarwindowmesh _cellarwindow_leftmesh _cellarwindow_centermesh _cellarwindow_rightmesh _doormesh _door_leftmesh _door_centermesh _door_rightmesh _door_arcmesh _windowmesh _window_leftmesh _window_centermesh _window_rightmesh) (break `/Game/Blueprints/Walls/Lists/WallMeshesStruct` _value))
  (return (select `bool` _returnvalue :`true` (select `/Game/Blueprints/Walls/Lists/WallTypes` WallType :`NewEnumerator22` _wallmesh :`NewEnumerator23` _wall_narrow01mesh :`NewEnumerator24` _wall_narrow02mesh :`NewEnumerator25` _wall_narrow03mesh :`NewEnumerator26` _wall_narrow04mesh :`NewEnumerator31` _wall_smallmesh :`NewEnumerator9` _balconymesh :`NewEnumerator10` _balcony_leftmesh :`NewEnumerator11` _balcony_centermesh :`NewEnumerator12` _balcony_rightmesh :`NewEnumerator13` _cellarwindowmesh :`NewEnumerator14` _cellarwindow_leftmesh :`NewEnumerator15` _cellarwindow_centermesh :`NewEnumerator16` _cellarwindow_rightmesh :`NewEnumerator17` _doormesh :`NewEnumerator18` _door_leftmesh :`NewEnumerator19` _door_centermesh :`NewEnumerator20` _door_rightmesh :`NewEnumerator21` _door_arcmesh :`NewEnumerator27` _windowmesh :`NewEnumerator28` _window_leftmesh :`NewEnumerator29` _window_centermesh :`NewEnumerator30` _window_rightmesh))))

(fn `SocketTypeToID`
  (params (Index :type "/Game/Blueprints/Walls/Lists/WallTypes Enum" :default "NewEnumerator8"))
  (returns (ID :type Integer))
  (return (select `/Game/Blueprints/Walls/Lists/WallTypes` Index :`NewEnumerator8` -1 :`NewEnumerator6` -1 :`NewEnumerator9` 1 :`NewEnumerator10` 2 :`NewEnumerator11` 2 :`NewEnumerator12` 2 :`NewEnumerator13` 3 :`NewEnumerator14` 4 :`NewEnumerator15` 4 :`NewEnumerator16` 4 :`NewEnumerator17` 5 :`NewEnumerator18` 6 :`NewEnumerator19` 6 :`NewEnumerator20` 6 :`NewEnumerator21` 7 :`NewEnumerator27` 8 :`NewEnumerator28` 9 :`NewEnumerator29` 9 :`NewEnumerator30` 9)))