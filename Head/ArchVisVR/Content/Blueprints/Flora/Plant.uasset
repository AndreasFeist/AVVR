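; Configurable potted plant actor that assembles pot, earth, saucer and plant meshes from asset lists in the construction script.
; The pot ID selects the matching earth type and decides whether the optional potplate is set up or its component destroyed.
; Earth and plant snap to pot sockets, with adjustable plant yaw.
; DynamicMaterialsController applies materials and colors to the pot and potplate.
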(fn `UserConstructionScript`
  (bind _potplate (`self.Potplate`))
  (bind _pot (`self.Pot`))
  (bind _plant (`self.Plant`))
  (bind _earth (`self.Earth`))
  (bind (_hasitems _mesh) (`/Game/Blueprints/Controller/AssetsFunctionLibrary.GetStaticMesh` (`self.Plants`) (`self.PlantID`)))
  (bind (_hasitems_2 _mesh_2 _id) (`/Game/Blueprints/Controller/AssetsFunctionLibrary.GetStaticMesh` (`self.Potplates`) (`self.PotplateID`)))
  (bind (_hasitems_3 _mesh_3 _id_2) (`/Game/Blueprints/Controller/AssetsFunctionLibrary.GetStaticMesh` (`self.Pots`) (`self.PotIDs`)))
  (bind _returnvalue (select `int` _id_2 :`0` 0 :`1` 0 :`2` 1 :`3` 1))
  (bind (_hasitems_4 _mesh_4) (`/Game/Blueprints/Controller/AssetsFunctionLibrary.GetStaticMesh` (`self.Earths`) _returnvalue))
  (if _hasitems_3
    (`StaticMeshComponent.SetStaticMesh` _pot _mesh_3)
    (`/Game/Blueprints/Controller/DynamicMaterialsController.SetupMaterial` (`self.DynamicMaterialsController`) (`self.PotMaterials`) _id_2 _pot 0 (`self.PotColor`))
    (`|ExecutionSequence`
      (:`then_0`
        (if _hasitems_4
          (`StaticMeshComponent.SetStaticMesh` _earth _mesh_4)
          (`SceneComponent.K2_AttachToComponent` _earth (`self.Pot`) "Earth" "SnapToTarget" "SnapToTarget" "KeepRelative" true)))
      (:`then_1`
        (if (and (== _returnvalue 0) (`self.UsePotplate`))
          (if _hasitems_2
            (`StaticMeshComponent.SetStaticMesh` _potplate _mesh_2)
            (`/Game/Blueprints/Controller/DynamicMaterialsController.SetupMaterial` (`self.DynamicMaterialsController`) (`self.PotPlateMaterials`) _id _potplate 0 (`self.PotplateColor`)))
          (else
            (`ActorComponent.K2_DestroyComponent` (`self.Potplate`)))))
      (:`then_2`
        (if _hasitems
          (`StaticMeshComponent.SetStaticMesh` _plant _mesh)
          (`SceneComponent.K2_AttachToComponent` _plant (`self.Pot`) "Plant" "SnapToTarget" "SnapToTarget" "KeepRelative" true)
          (`SceneComponent.K2_AddLocalRotation` _plant (`KismetMathLibrary.MakeRotator` 0.0 0.0 (`self.PlantYaw`)) false false))))))