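; Configurable TV prop Blueprint that builds its appearance and audio setup in the Construction Script.
; TVID selects a mesh from the TVSets list, and all setup is skipped when the lookup returns no items.
; DynamicMaterialsController applies the TVID material from TVMaterials with MeshColor to that mesh.
; TVScreenController sets up TVAudio on the TV component using the actor's AudioProperties.
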(fn `UserConstructionScript`
  (bind _tv (`self.TV`))
  (bind _tvid (`self.TVID`))
  (bind (_hasitems _mesh) (`/Game/Blueprints/Controller/AssetsFunctionLibrary.GetStaticMesh` (`self.TVSets`) _tvid))
  (if _hasitems
    (`StaticMeshComponent.SetStaticMesh` _tv _mesh)
    (`/Game/Blueprints/Controller/DynamicMaterialsController.SetupMaterial` (`self.DynamicMaterialsController`) (`self.TVMaterials`) _tvid _tv 0 (`self.MeshColor`))
    (`/Game/Blueprints/Controller/TVScreenController.SetupAudio` (`self.TVScreenController`) (`self.TVAudio`) _tv (`self.AudioProperties`))))