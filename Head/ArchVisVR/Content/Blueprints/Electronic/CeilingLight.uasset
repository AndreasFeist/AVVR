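; Ceiling light Blueprint that configures its lamp mesh, material and point light in the construction script.
; It looks up a mesh in the CeilingLamps asset list by LampID and proceeds only if the lookup returns items.
; DynamicMaterialsController applies the material for the same ID with MeshColor, then LightController sets up the point light from LightProperties with the lamp as attach component.
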(fn `UserConstructionScript`
  (bind _lamp (`self.Lamp`))
  (bind _lampid (`self.LampID`))
  (bind (_hasitems _mesh) (`/Game/Blueprints/Controller/AssetsFunctionLibrary.GetStaticMesh` (`self.CeilingLamps`) _lampid))
  (if _hasitems
    (`StaticMeshComponent.SetStaticMesh` _lamp _mesh)
    (`/Game/Blueprints/Controller/DynamicMaterialsController.SetupMaterial` (`self.DynamicMaterialsController`) (`self.LampMaterials`) _lampid _lamp 0 (`self.MeshColor`))
    (`/Game/Blueprints/Controller/LightController.SetupLight` (`self.LightController`) (`self.PointLight`) (`self.Lamp`) (`self.LightProperties`))))