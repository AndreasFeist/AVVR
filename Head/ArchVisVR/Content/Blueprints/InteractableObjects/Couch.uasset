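; Interactable-object couch Blueprint that configures its mesh and look in the construction script.
; CouchID picks the static mesh from the Couches asset list and also serves as the material ID for CouchMaterials.
; If the lookup has items, it sets the mesh, then DynamicMaterialsController sets up the material with CouchColor and applies a fuzz color to the first material slot.
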(fn `UserConstructionScript`
  (bind _couch (`self.Couch`))
  (bind _couchid (`self.CouchID`))
  (bind _dynamicmaterialscontroller (`self.DynamicMaterialsController`))
  (bind (_hasitems _mesh) (`/Game/Blueprints/Controller/AssetsFunctionLibrary.GetStaticMesh` (`self.Couches`) _couchid))
  (if _hasitems
    (`StaticMeshComponent.SetStaticMesh` _couch _mesh)
    (`/Game/Blueprints/Controller/DynamicMaterialsController.SetupMaterial` _dynamicmaterialscontroller (`self.CouchMaterials`) _couchid _couch 0 (`self.CouchColor`))
    (`/Game/Blueprints/Controller/DynamicMaterialsController.SetFuzzColor` _dynamicmaterialscontroller 0 (`self.CouchFuzzColor`))))