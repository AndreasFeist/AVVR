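; Base Blueprint for a combined floor and ceiling piece with a selectable mesh, materials and colors.
; The construction script looks up a mesh in the Floors list by FloorID and, if found, assigns it to the Floor component.
; SetupMaterials then passes each material slot to DynamicMaterialsController with its own material ID and color, drawing from floor materials for the first slot and ceiling materials for the second.
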(fn `SetupMaterials`
  (params (Mesh :type "MeshComponent Object Reference"))
  (for (_ _array_index) (`MeshComponent.GetMaterials` Mesh)
    (`/Game/Blueprints/Controller/DynamicMaterialsController.SetupMaterial` (`self.DynamicMaterialsController`) (select `int` _array_index :`0` (`self.FloorMaterials`) :`1` (`self.CeilingMaterials`)) (`|GetArrayItem` (`self.MeshMaterials`) _array_index) Mesh _array_index (`|GetArrayItem` (`self.Color`) _array_index))))

(fn `UserConstructionScript`
  (bind _floor (`self.Floor`))
  (bind (_hasitems _mesh) (`/Game/Blueprints/Controller/AssetsFunctionLibrary.GetStaticMesh` (`self.Floors`) (`self.FloorID`)))
  (if _hasitems
    (`StaticMeshComponent.SetStaticMesh` _floor _mesh)
    (`self.SetupMaterials` _floor)))