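; Base wall Blueprint that builds a modular wall along a linearized spline in its construction script.
; It creates one instanced static mesh component per wall type, with materials set through DynamicMaterialsController, including optional front/back blending and a separate cap-off.
; Segment count comes from spline length over mesh length, resizing the editable segment-type list while keeping existing choices.
; Each segment becomes an instance at its spline distance, and matching socket transforms are collected per socket type.
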(fn `GetMaterialBlendVectors`
  (params (ID :type Integer))
  (returns (BottomLeft :type "Vector Structure") (TopRight :type "Vector Structure"))
  (bind _returnvalue (`self.GetTransform` self))
  (return (select `int` ID :`0` (`KismetMathLibrary.TransformLocation` _returnvalue (`self.FrontSite_BottomLeft`)) :`1` (`KismetMathLibrary.TransformLocation` _returnvalue (`self.BackSite_BottomLeft`))) (select `int` ID :`0` (`KismetMathLibrary.TransformLocation` _returnvalue (`self.ForntSite_TopRight`)) :`1` (`KismetMathLibrary.TransformLocation` _returnvalue (`self.BackSite_TopRight`)))))

(fn `SetLinearSplinePoints`
  (bind _spline (`self.Spline`))
  (for _index (range (`SplineComponent.GetNumberOfSplinePoints` _spline))
    (`SplineComponent.SetSplinePointType` _spline _index "Linear" false))
  (`SplineComponent.UpdateSpline` _spline))

(fn `SetupInstanceMeshComponents`
  (for _array_element (`self.WallTypes`)
    (bind _returnvalue (`AddComponent|NODE_AddInstancedStaticMeshComponent-0`))
    (`StaticMeshComponent.SetStaticMesh` _returnvalue (`/Game/Blueprints/Controller/AssetsFunctionLibrary.GetWallMesh` _array_element (`self.WallMeshesMap`) (`self.WallHeight`)))
    (`self.SetupMaterials` _returnvalue)
    (`BlueprintMapLibrary.Map_Add` (`self.WallsInstanceMeshesMap`) _array_element _returnvalue)))

(fn `SetupMaterials`
  (params (Mesh :type "MeshComponent Object Reference"))
  (bind _dynamicmaterialscontroller (`self.DynamicMaterialsController`))
  (for (_ _array_index) (`MeshComponent.GetMaterials` Mesh)
    (bind _output (`|GetArrayItem` (`self.UseBlend`) _array_index))
    (bind _returnvalue (== _array_index 2))
    (`/Game/Blueprints/Controller/DynamicMaterialsController.SetupMaterial` _dynamicmaterialscontroller (select `bool` _returnvalue :`false` (select `bool` _output :`false` (`self.WallMaterials_noBlend`) :`true` (`self.WallMaterials_Blend`)) :`true` (`self.WallMaterialsCapoff`)) (`|GetArrayItem` (`self.WallMaterialID`) _array_index) Mesh _array_index (select `bool` _returnvalue :`false` (`KismetMathLibrary.SelectColor` (struct :`R` 1.0 :`G` 1.0 :`B` 1.0 :`A` 1.0) (`|GetArrayItem` (`self.WallInnerColor`) _array_index) _output) :`true` (`|GetArrayItem` (`self.WallInnerColor`) _array_index)))
    (if (and (!= _array_index 2) _output)
      (bind (_bottomleft _topright) (`self.GetMaterialBlendVectors` _array_index))
      (`/Game/Blueprints/Controller/DynamicMaterialsController.SetMaterialBlendValues` _dynamicmaterialscontroller _array_index (`|GetArrayItem` (`self.WallMaterialParameters`) _array_index) (`|GetArrayItem` (`self.WallInnerColor`) _array_index) (`|GetArrayItem` (`self.WallOuterColor`) _array_index) _bottomleft _topright))))

(fn `SetupSocketList`
  (params (InstanceMeshComponent :type "InstancedStaticMeshComponent Object Reference") (WallType :type "/Game/Blueprints/Walls/Lists/WallTypes Enum" :default "NewEnumerator8") (TransformAlongSpline :type "Transform Structure"))
  (bind _id (`/Game/Blueprints/Controller/AssetsFunctionLibrary.SocketTypeToID` WallType))
  (bind (_socketname _transforms) (break `/Game/Blueprints/Walls/Lists/WallSockets` (`|GetArrayItem` (`self.Sockets`) _id)))
  (if (and (>= _id 0) (`SceneComponent.DoesSocketExist` InstanceMeshComponent _socketname))
    (`KismetArrayLibrary.Array_AddUnique` _transforms (`KismetMathLibrary.ComposeTransforms` TransformAlongSpline (`SceneComponent.GetSocketTransform` InstanceMeshComponent _socketname "RTS_World")))))

(fn `SetupWalls`
  (locals (MeshLength :type "Float (double-precision)") (NumberOfMeshes :type Integer :default 0) (TestType :type "/Game/Blueprints/Walls/Lists/WallTypes Enum" :default "NewEnumerator8") (CurrentWallSegments :type "Array of /Game/Blueprints/Walls/Lists/WallTypes Enum") (SocketNames :type "Array of Name"))
  (bind _testtype (`local.TestType`))
  (bind _wallsegments (`self.WallSegments`))
  (bind _returnvalue (`StaticMesh.GetBoundingBox` (`.WallMesh_8_2A5CD1AA4578DC91480E5C8C896B9801` (break `/Game/Blueprints/Walls/Lists/WallMeshesStruct` (`BlueprintMapLibrary.Map_Find` (`self.WallMeshesMap`) (`self.WallHeight`))))))
  (bind _returnvalue_2 (select `ESplineMeshAxis` (`self.Axis`) :`X` (.x (`.Max` (break `Box` _returnvalue))) :`Y` (.y (`.Max` (break `Box` _returnvalue))) :`Z` (.z (`.Max` (break `Box` _returnvalue)))))
  (set `local.MeshLength` _returnvalue_2)
  (set `local.NumberOfMeshes` (- (`.ReturnValue` (`KismetMathLibrary.FMod` (`SplineComponent.GetSplineLength` (`self.Spline`)) _returnvalue_2)) 1))
  (`|ExecutionSequence`
    (:`then_0`
      (`KismetArrayLibrary.Array_Clear` (`self.Sockets`))
      (for _array_element (`local.SocketNames`)
        (`KismetArrayLibrary.Array_Add` (`self.Sockets`) (make `/Game/Blueprints/Walls/Lists/WallSockets` _array_element (`|MakeArray`)))))
    (:`then_1`
      (for _index (range (+ (`local.NumberOfMeshes`) 1))
        (bind _output (`|GetArrayItem` (`self.WallSegments`) _index))
        (`KismetArrayLibrary.Array_Set` (`local.CurrentWallSegments`) _index (select `bool` (`|EnumInequality` _output _testtype) :`false` _testtype :`true` _output) true))
      (`KismetArrayLibrary.Array_Clear` _wallsegments)
      (`KismetArrayLibrary.Array_Append` _wallsegments (`local.CurrentWallSegments`)))
    (:`then_2`
      (for (_array_element_2 _array_index) (`self.WallSegments`)
        (bind (_value _returnvalue_3) (`BlueprintMapLibrary.Map_Find` (`self.WallsInstanceMeshesMap`) _array_element_2))
        (if _returnvalue_3
          (bind _returnvalue_4 (`SplineComponent.GetTransformAtDistanceAlongSpline` (`self.Spline`) (* _array_index (`local.MeshLength`)) "Local" false))
          (`InstancedStaticMeshComponent.AddInstance` _value _returnvalue_4)
          (`self.SetupSocketList` _value _array_element_2 _returnvalue_4))))))

(fn `UserConstructionScript`
  (set `self.DEBUG` false)
  (`self.SetupInstanceMeshComponents`)
  (`self.SetLinearSplinePoints`)
  (`self.SetupWalls`))