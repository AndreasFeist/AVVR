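; Base door actor that asks its DoorController to interact when player pawn 0 begins overlapping it.
; The construction script builds the door from mesh arrays, picking frame, panel and skeletal grip by ID.
; IsLeft switches between left and right meshes, grip anim instance classes and the anchor that positions panel and grip.
; It also sizes the Sphere component from DoorSphereRadius.
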(event `self.ReceiveActorBeginOverlap`
  (params (OtherActor :type "Actor Object Reference"))
  (if (== OtherActor (`GameplayStatics.GetPlayerPawn` 0))
    (`/Game/Blueprints/Controller/DoorController.InteractWithDoor` (`self.DoorController`))))

(fn `UserConstructionScript`
  (bind _isleft (`self.IsLeft`))
  (bind _door (`self.Door`))
  (bind _doorgrip (`self.DoorGrip`))
  (bind _doorgripid (`self.DoorGripID`))
  (bind _relativelocation (`SceneComponent.RelativeLocation` (select `bool` (`self.IsLeft`) :`false` (`self.DoorRightAnchor`) :`true` (`self.DoorLeftAnchor`))))
  (`StaticMeshComponent.SetStaticMesh` (`self.DoorFrame`) (`|GetArrayItem` (`self.DoorFrameMeshes`) (`self.DoorFrameID`)))
  (`StaticMeshComponent.SetStaticMesh` _door (`|GetArrayItem` (select `bool` (`self.IsLeft`) :`false` (`self.DoorRightMeshes`) :`true` (`self.DoorLeftMeshes`)) (`self.DoorID`)))
  (`SceneComponent.K2_SetRelativeLocation` _door _relativelocation false false)
  (`SkinnedMeshComponent.SetSkinnedAssetAndUpdate` _doorgrip (`|GetArrayItem` (select `bool` _isleft :`false` (`self.DoorGripRightMeshes`) :`true` (`self.DoorGripLeftMeshes`)) _doorgripid) true)
  (`SkeletalMeshComponent.SetAnimInstanceClass` _doorgrip (`|GetArrayItem` (select `bool` _isleft :`false` (`self.DoorGripRightAnimInstances`) :`true` (`self.DoorGripLightAnimInstances`)) _doorgripid))
  (`SceneComponent.K2_SetRelativeLocation` _doorgrip _relativelocation false false)
  (`SphereComponent.SetSphereRadius` (`self.Sphere`) (`self.DoorSphereRadius`) true))