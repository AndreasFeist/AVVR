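; WallBase is a building wall piece that sets its static mesh at construction from its wall type.
; It reads the parent Walls actor's height and looks up the type's row in the mid table for medium, or the high table for short, high and no Walls parent.
; The row supplies the mesh and a socket name, used to reposition an attached WallObject when the row's object type calls for one.
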(fn `SetupWall`
  (locals (WallStruct :type "/Game/Blueprints/Buildings/WallStruct Structure"))
  (bind _wallobject (`self.WallObject`))
  (bind _staticmesh (`self.StaticMesh`))
  (bind (_wallmesh _socketname _wallobject_2) (break `/Game/Blueprints/Buildings/WallStruct` (`local.WallStruct`)))
  (bind _returnvalue (`KismetStringLibrary.Conv_StringToName` (`|GetEnumeratorNameAsString` (`self.WallType`))))
  (bind _aswalls (cast `/Game/Blueprints/Buildings/Walls` (`self.GetParentActor` self))
    (:`then`
      (switch `/Game/Blueprints/Buildings/WallHeight` (`/Game/Blueprints/Buildings/Walls.WallHeight` _aswalls)
        (:`NewEnumerator5`
          (bind _returnvalue_2 (`|GetDataTableRow` "/Game/Blueprints/Buildings/WallsHighDataTable.WallsHighDataTable" _returnvalue)
            (:`then`
              (set `local.WallStruct` _returnvalue_2))))
        (:`NewEnumerator6`
          (bind _returnvalue_3 (`|GetDataTableRow` "/Game/Blueprints/Buildings/WallsMidDataTable.WallsMidDataTable" _returnvalue)
            (:`then`
              (set `local.WallStruct` _returnvalue_3))))
        (:`NewEnumerator7`
          (bind _returnvalue_4 (`|GetDataTableRow` "/Game/Blueprints/Buildings/WallsHighDataTable.WallsHighDataTable" _returnvalue)
            (:`then`
              (set `local.WallStruct` _returnvalue_4))))))
    (:`CastFailed`
      (bind _returnvalue_5 (`|GetDataTableRow` "/Game/Blueprints/Buildings/WallsHighDataTable.WallsHighDataTable" _returnvalue)
        (:`then`
          (set `local.WallStruct` _returnvalue_5)))))
  (`StaticMeshComponent.SetStaticMesh` _staticmesh _wallmesh)
  (if (`|EnumInequality` _wallobject_2 "NewEnumerator9")
    (if (!= null _wallobject)
      (`self.K2_SetActorTransform` _wallobject (`SceneComponent.GetSocketTransform` _staticmesh _socketname "RTS_World") false false))))

(fn `UserConstructionScript`
  (locals (WallStruct :type "/Game/Blueprints/Buildings/WallStruct Structure"))
  (`self.SetupWall`))