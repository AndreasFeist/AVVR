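; Spline-based modular wall builder that lays WallBase child actors along a spline from the construction script.
; CreateWalls derives segment count and spacing from spline length and each segment's mesh bounds.
; Per-segment type and object arrays configure each piece through SetupWall, with fallback defaults, and are resized to the segment count.
; ClearWalls destroys the segments, resets the spline to a short straight line and rebuilds.
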(event `ClearWalls`
  (bind _wallsegments (`self.WallSegments`))
  (`ActorComponent.K2_DestroyComponent` _wallsegments)
  (`KismetArrayLibrary.Array_Clear` _wallsegments)
  (`KismetArrayLibrary.Array_Clear` (`self.WallSegmentTypes`))
  (`SplineComponent.SetSplinePoints` (`self.Spline`) (`|MakeArray` (0.0 0.0 0.0) (150.0 0.0 0.0) :!type "Vector Structure") "Local" true)
  (`self.CreateWalls`))

(fn `CreateWalls`
  (locals (LastSegment :type "Float (double-precision)") (Length :type "Float (double-precision)" :default 0.0) (Index :type Integer))
  (bind _wallsegmenttypes (`self.WallSegmentTypes`))
  (bind _wallobject (`self.WallObject`))
  (bind _index (`local.Index`))
  (bind _spline (`self.Spline`))
  (bind _returnvalue (+ (`local.Index`) 1))
  (bind _output (`|GetArrayItem` _wallsegmenttypes))
  (bind _output_2 (`|GetArrayItem` _wallobject))
  (bind _output_3 (`|GetArrayItem` (`self.WallSegmentTypes`) _returnvalue))
  (bind _output_4 (`|GetArrayItem` (`self.WallObject`) _returnvalue))
  (bind _returnvalue_2 (+ _index (select `bool` (!= _index 0) :`false` 1 :`true` 2)))
  (bind _returnvalue_3 (select `bool` (`|EnumInequality` _output_3 "NewEnumerator6") :`false` "NewEnumerator0" :`true` _output_3))
  (bind _returnvalue_4 (select `bool` (!= _output_4 null) :`true` _output_4))
  (`|ExecutionSequence`
    (:`then_0`
      (`KismetArrayLibrary.Array_Set` _wallsegmenttypes 0 (select `bool` (`|EnumInequality` _output "NewEnumerator6") :`false` "NewEnumerator0" :`true` _output) true))
    (:`then_1`
      (`KismetArrayLibrary.Array_Set` _wallobject 0 (select `bool` (!= _output_2 null) :`true` _output_2) true)
      (bind _returnvalue_5 (`AddComponent|NODE_AddChildActorComponent-3`))
      (bind _aswall_base (cast `/Game/Blueprints/Buildings/WallBase` (`ChildActorComponent.ChildActor` _returnvalue_5)))
      (set `/Game/Blueprints/Buildings/WallBase.WallType` (`|GetArrayItem` (`self.WallSegmentTypes`)) _aswall_base)
      (set `/Game/Blueprints/Buildings/WallBase.WallObject` (`|GetArrayItem` (`self.WallObject`)) _aswall_base)
      (`/Game/Blueprints/Buildings/WallBase.SetupWall` _aswall_base)
      (bind _x (.x (`.Max` (`StaticMeshComponent.GetLocalBounds` (`/Game/Blueprints/Buildings/WallBase.StaticMesh` _aswall_base)))))
      (`SceneComponent.K2_SetRelativeTransform` _returnvalue_5 (`SplineComponent.GetTransformAtDistanceAlongSpline` (`self.Spline`) _x "Local" true) false false)
      (`KismetArrayLibrary.Array_Set` (`self.WallSegments`) 0 _returnvalue_5 true)
      (bind _returnvalue_6 (* _x 2.0))
      (set `local.Length` (+ _x _returnvalue_6))
      (for _index_2 (range (`.ReturnValue` (`KismetMathLibrary.FMod` (- (`SplineComponent.GetSplineLength` _spline) _x) _returnvalue_6)))
        (set `local.Index` _index_2)
        (bind _returnvalue_7 (`AddComponent|NODE_AddChildActorComponent-2` :`RelativeTransform` (`SplineComponent.GetTransformAtDistanceAlongSpline` _spline (`local.Length`) "Local" true)))
        (`KismetArrayLibrary.Array_Set` (`self.WallSegments`) _returnvalue _returnvalue_7 true)
        (bind _aswall_base_2 (cast `/Game/Blueprints/Buildings/WallBase` (`ChildActorComponent.ChildActor` _returnvalue_7)))
        (`KismetArrayLibrary.Array_Set` (`self.WallSegmentTypes`) _returnvalue _returnvalue_3 true)
        (`KismetArrayLibrary.Array_Set` (`self.WallObject`) _returnvalue _returnvalue_4)
        (set `/Game/Blueprints/Buildings/WallBase.WallType` _returnvalue_3 _aswall_base_2)
        (set `/Game/Blueprints/Buildings/WallBase.WallObject` _returnvalue_4 _aswall_base_2)
        (`/Game/Blueprints/Buildings/WallBase.SetupWall` _aswall_base_2)
        (set `local.Length` (+ (`local.Length`) (* (.x (`.Max` (`StaticMeshComponent.GetLocalBounds` (`/Game/Blueprints/Buildings/WallBase.StaticMesh` _aswall_base_2)))) 2.0))))
      (`KismetArrayLibrary.Array_Resize` (`self.WallSegments`) _returnvalue_2)
      (`KismetArrayLibrary.Array_Resize` (`self.WallSegmentTypes`) _returnvalue_2)
      (`KismetArrayLibrary.Array_Resize` (`self.WallObject`) _returnvalue_2))))

(fn `UserConstructionScript`
  (`self.CreateWalls`))