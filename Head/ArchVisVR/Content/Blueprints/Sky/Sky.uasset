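; Sky actor that configures a level's lighting, fog and sky from exposed variables in its construction script.
; Init functions set up the skylight, directional light, exponential height fog and atmospheric fog, destroying any component whose toggle is off.
; The sky sphere gets a dynamic material chosen by SkyType (color, cubemap, or cloud-and-star domes), optionally inheriting skylight cubemap and sun color.
; It also writes main light direction and global specular into a material parameter collection.
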(fn `AmbientSkyLightInit`
  (bind _ambientskylight (`self.AmbientSkyLight`))
  (if (`self.UseAmbientSkyLight`)
    (`SkyLightComponent.SetIntensity` _ambientskylight (`self.AmbientIntensity`))
    (`SkyLightComponent.SetIndirectLightingIntensity` _ambientskylight (`self.AmbientIndirectLightingIntensity`))
    (`SkyLightComponent.SetVolumetricScatteringIntensity` _ambientskylight (`self.AmbientVolumetricScatteringIntensity`))
    (`SkyLightComponent.SetOcclusionTint` _ambientskylight (`self.AmbientTintColor`))
    (`SkyLightComponent.SetCubemap` _ambientskylight (`self.AmbientCubemap`))
    (else
      (`ActorComponent.K2_DestroyComponent` (`self.AmbientSkyLight`)))))

(fn `AtmosphericFogInit`
  (bind _atmosphericfog (`self.AtmosphericFog`))
  (bind _atmosphericfog_2 (`self.AtmosphericFog`))
  (if (`self.UseAtmosphericFog`)
    (`|ExecutionSequence`
      (:`then_0`
        ;[1 1 1] Atmosphere settings
        (`AtmosphericFogComponent.SetSunMultiplier` _atmosphericfog (`self.AtmosphericFogSunMultiplier`))
        (`AtmosphericFogComponent.SetFogMultiplier` _atmosphericfog (`self.AtmosphericFogMultiplier`))
        (`AtmosphericFogComponent.SetDensityMultiplier` _atmosphericfog (`self.AtmosphericFogDensityMultiplier`))
        (`AtmosphericFogComponent.SetDensityOffset` _atmosphericfog (`self.AtmosphericFogDensityOffset`))
        (`AtmosphericFogComponent.SetDistanceScale` _atmosphericfog (`self.AtmosphericFogDistanceScale`))
        (`AtmosphericFogComponent.SetAltitudeScale` _atmosphericfog (`self.AtmosphericFogAltitudeScale`))
        (`AtmosphericFogComponent.SetDistanceOffset` _atmosphericfog (`self.AtmosphericFogDistanceOffset`))
        (set `AtmosphericFogComponent.GroundOffset` (`self.AtmosphericFogGroundOffset`) _atmosphericfog)
        (`AtmosphericFogComponent.SetStartDistance` _atmosphericfog (`self.AtmosphericFogStartDistance`))
        (set `AtmosphericFogComponent.SunDiscScale` (`self.AtmosphericFogSunDiscScale`) _atmosphericfog))
      (:`then_1`
        ;[1 1 1] Lighting settings
        (`AtmosphericFogComponent.SetDefaultBrightness` _atmosphericfog_2 (`self.AtmosphericFogDefaultBrightness`))
        (`AtmosphericFogComponent.SetDefaultLightColor` _atmosphericfog_2 (`self.AtmosphericFogDefaultLightColor`))
        (`AtmosphericFogComponent.DisableSunDisk` _atmosphericfog_2 (`self.AtmosphericFogDisableSunDisk`))
        (`AtmosphericFogComponent.DisableGroundScattering` _atmosphericfog_2 (`self.AtmosphericFogDisableGroundScattering`))))
    (else
      (`ActorComponent.K2_DestroyComponent` (`self.AtmosphericFog`)))))

(fn `DirectionalLightInit`
  (bind _mainlight (`self.MainLight`))
  (bind _mainlight_2 (`self.MainLight`))
  (bind _mainlight_3 (`self.MainLight`))
  (bind _mainlight_4 (`self.MainLight`))
  (if (`self.UseMainLight`)
    (`|ExecutionSequence`
      (:`then_0`
        ;[1 1 1] Light settings
        (`SceneComponent.K2_SetRelativeRotation` _mainlight (`self.MainLightRotation`) false false)
        (`LightComponent.SetIntensity` _mainlight (`self.MainLightIntensity`))
        (`LightComponent.SetLightColor` _mainlight (`self.MainLightColor`) true)
        (`LightComponent.SetIndirectLightingIntensity` _mainlight (`self.MainLightIndirectLightingIntensity`))
        (`LightComponent.SetVolumetricScatteringIntensity` _mainlight (`self.MainLightVolumetricScatteringIntensity`)))
      (:`then_1`
        ;[1 1 1] Light Shaft settings
        (`DirectionalLightComponent.SetOcclusionMaskDarkness` _mainlight_2 (`self.MainLightOcclusionMaskDarkness`))
        (`LightComponent.SetBloomScale` _mainlight_2 (`self.MainLightBloomScale`))
        (`LightComponent.SetBloomThreshold` _mainlight_2 (`self.MainLightBloomThreshold`))
        (`LightComponent.SetBloomTint` _mainlight_2 (`self.MainLightBloomTint`)))
      (:`then_2`
        ;[1 1 1] Shadow Casting
        (`DirectionalLightComponent.SetDynamicShadowCascades` _mainlight_3 (`self.MainLightShadowCascades`))
        (`DirectionalLightComponent.SetCascadeDistributionExponent` _mainlight_3 (`self.MainLightCascadeDistributionExponent`))
        (`DirectionalLightComponent.SetCascadeTransitionFraction` _mainlight_3 (`self.MainLightCascadeTransitionFraction`)))
      (:`then_3`
        ;[1 1 1] Light Function Settings
        (`LightComponent.SetLightFunctionMaterial` _mainlight_4 (`self.MainLightLightFunction`))
        (`LightComponent.SetLightFunctionScale` _mainlight_4 (`self.MainLightLightFunctionScale`))
        (`LightComponent.SetLightFunctionFadeDistance` _mainlight_4 (`self.MainLightLightFunctionFadeDistance`))
        (`LightComponent.SetLightFunctionDisabledBrightness` _mainlight_4 (`self.MainLightLightFunctionDisabledBrightness`))))
    (else
      (`ActorComponent.K2_DestroyComponent` (`self.MainLight`)))))

(fn `ExponentialHeightFogInit`
  (bind _exponentialheightfog (`self.ExponentialHeightFog`))
  (bind _exponentialfogusevolumetricfog (`self.ExponentialFogUseVolumetricFog`))
  (bind _exponentialheightfog_2 (`self.ExponentialHeightFog`))
  (bind _exponentialheightfog_3 (`self.ExponentialHeightFog`))
  (bind _exponentialheightfog_4 (`self.ExponentialHeightFog`))
  (if (`self.UseExponentialFog`)
    (`|ExecutionSequence`
      (:`then_0`
        ;[1 1 1] Height Fog settings
        (`ExponentialHeightFogComponent.SetFogDensity` _exponentialheightfog_2 (`self.ExponentialFogDensity`))
        (`ExponentialHeightFogComponent.SetFogInscatteringColor` _exponentialheightfog_2 (`self.ExponentialFogInscatteringColor`))
        (`ExponentialHeightFogComponent.SetFogHeightFalloff` _exponentialheightfog_2 (`self.ExponentialFogHeightFalloff`))
        (`ExponentialHeightFogComponent.SetFogMaxOpacity` _exponentialheightfog_2 (`self.ExponentialFogMaxOpacity`))
        (`ExponentialHeightFogComponent.SetStartDistance` _exponentialheightfog_2 (`self.ExponentialFogStartDistance`))
        (`ExponentialHeightFogComponent.SetFogCutoffDistance` _exponentialheightfog_2 (`self.ExponentialFogCutoffDistance`)))
      (:`then_1`
        ;[1 1 1] Inscattering Texture
        (`ExponentialHeightFogComponent.SetInscatteringColorCubemap` _exponentialheightfog_4 (`self.ExponentialFogInscatteringColorCubemap`))
        (`ExponentialHeightFogComponent.SetInscatteringColorCubemapAngle` _exponentialheightfog_4 (`self.ExponentialFogInscatteringColorCubemapAngle`))
        (`ExponentialHeightFogComponent.SetInscatteringTextureTint` _exponentialheightfog_4 (`self.ExponentialFogInscatteringTextureTint`)))
      (:`then_2`
        ;[1 1 1] Directional Inscattering settings
        (`ExponentialHeightFogComponent.SetDirectionalInscatteringExponent` _exponentialheightfog_3 (`self.ExponentialFogDirectionalInscatteringExponent`))
        (`ExponentialHeightFogComponent.SetDirectionalInscatteringStartDistance` _exponentialheightfog_3 (`self.ExponentialFogDirectionalInscatteringStartDistance`))
        (`ExponentialHeightFogComponent.SetDirectionalInscatteringColor` _exponentialheightfog_3 (`self.ExponentialFogDirectioanlInscatteringColor`)))
      (:`then_3`
        ;[1 1 1] Volumetric Fog settings
        (`ExponentialHeightFogComponent.SetVolumetricFog` _exponentialheightfog _exponentialfogusevolumetricfog)
        (if _exponentialfogusevolumetricfog
          (`ExponentialHeightFogComponent.SetVolumetricFogScatteringDistribution` _exponentialheightfog (`self.ExponentialFogVolumetricFogScatteringDistribution`))
          (`ExponentialHeightFogComponent.SetVolumetricFogAlbedo` _exponentialheightfog (`self.ExponentialFogVolumetricFogAlbedo`))
          (`ExponentialHeightFogComponent.SetVolumetricFogEmissive` _exponentialheightfog (`self.ExponentialFogVolumetricFogEmissive`))
          (`ExponentialHeightFogComponent.SetVolumetricFogExtinctionScale` _exponentialheightfog (`self.ExponentialFogVolumetricExtinctionScale`)))))
    (else
      (`ActorComponent.K2_DestroyComponent` (`self.ExponentialHeightFog`)))))

(fn `MaterialParameterCollectionInit`
  (bind _mainlight (`self.MainLight`))
  (`KismetMaterialLibrary.SetVectorParameterValue` "/Game/Materials/ParameterCollections/GlobalCollections.GlobalCollections" "SpecularParameters" (`self.GlobalSpecular`))
  (`/Engine/EditorBlueprintResources/StandardMacros.IsValid` _mainlight
    (:`Is Valid`
      (`KismetMaterialLibrary.SetVectorParameterValue` "/Game/Materials/ParameterCollections/GlobalCollections.GlobalCollections" "MainLightDirection" (`KismetMathLibrary.Conv_VectorToLinearColor` (`KismetMathLibrary.Conv_RotatorToVector` (`SceneComponent.K2_GetComponentRotation` _mainlight)))))))

(fn `SkySphereInit`
  (bind _skyspherematerial (`self.SkySphereMaterial`))
  (bind _skyspherematerial_2 (`self.SkySphereMaterial`))
  (bind _skyspherematerial_3 (`self.SkySphereMaterial`))
  (bind _skyspherematerial_4 (`self.SkySphereMaterial`))
  (bind _skyspherematerial_5 (`self.SkySphereMaterial`))
  (bind _skyspherematerial_6 (`self.SkySphereMaterial`))
  (if (`self.UseSkySphere`)
    (bind _returnvalue (`PrimitiveComponent.CreateDynamicMaterialInstance` (`self.SkySphere`) 0 (`BlueprintMapLibrary.Map_Find` (`self.SkySphereMaterials`) (`self.SkyType`))))
    (set `self.SkySphereMaterial` _returnvalue)
    (switch `/Game/Blueprints/Sky/Lists/SkySphereMaterials` (`self.SkyType`)
      (:`NewEnumerator0`
        (`MaterialInstanceDynamic.SetVectorParameterValue` (`self.SkySphereMaterial`) "BaseColor" (`self.BaseColor`)))
      (:`NewEnumerator1`
        (`MaterialInstanceDynamic.SetVectorParameterValue` _skyspherematerial "BaseColor" (`self.BaseColor`))
        (if (`self.UseAmbientSkyLight`)
          (set `self.Cubemap` (`self.AmbientCubemap`)))
        (`MaterialInstanceDynamic.SetTextureParameterValue` _skyspherematerial "Cubemap" (`self.Cubemap`)))
      (:`NewEnumerator2`
        (`MaterialInstanceDynamic.SetVectorParameterValue` _skyspherematerial_2 "BaseColor" (`self.BaseColor`))
        (`MaterialInstanceDynamic.SetScalarParameterValue` _skyspherematerial_2 "CloudsIntensity" (`self.CloudsIntensity`) :!label _label)
        (`MaterialInstanceDynamic.SetVectorParameterValue` _skyspherematerial_2 "CloudsColor" (`self.CloudsColor`))
        (`|ExecutionSequence`
          (:`then_0`
            (`MaterialInstanceDynamic.SetTextureParameterValue` _skyspherematerial_3 "CloudsMask01" (`self.CloudsMask01`))
            (`MaterialInstanceDynamic.SetScalarParameterValue` _skyspherematerial_3 "CloudsMask01TilingU" (`self.CloudsMask01TilingU`))
            (`MaterialInstanceDynamic.SetScalarParameterValue` _skyspherematerial_3 "CloudsMask01TilingV" (`self.CloudsMask01TilingV`))
            (`MaterialInstanceDynamic.SetScalarParameterValue` _skyspherematerial_3 "CloudsMask01SpeedU" (`self.CloudsMask01SpeedU`))
            (`MaterialInstanceDynamic.SetScalarParameterValue` _skyspherematerial_3 "CloudsMask01SpeedV" (`self.CloudsMask01SpeedV`))
            (`MaterialInstanceDynamic.SetScalarParameterValue` _skyspherematerial_3 "CloudsMask01SmoothStepMin" (`self.CloudsMask01SmoothStepMin`))
            (`MaterialInstanceDynamic.SetScalarParameterValue` _skyspherematerial_3 "CloudsMask01SmoothStepRange" (`self.CloudsMask01SmoothStepRange`)))
          (:`then_1`
            (`MaterialInstanceDynamic.SetTextureParameterValue` _skyspherematerial_4 "CloudsMask02" (`self.CloudsMask02`))
            (`MaterialInstanceDynamic.SetScalarParameterValue` _skyspherematerial_4 "CloudsMask02TilingU" (`self.CloudsMask02TilingU`))
            (`MaterialInstanceDynamic.SetScalarParameterValue` _skyspherematerial_4 "CloudsMask02TilingV" (`self.CloudsMask02TilingV`))
            (`MaterialInstanceDynamic.SetScalarParameterValue` _skyspherematerial_4 "CloudsMask02SpeedU" (`self.CloudsMask02SpeedU`))
            (`MaterialInstanceDynamic.SetScalarParameterValue` _skyspherematerial_4 "CloudsMask02SpeedV" (`self.CloudsMask02SpeedV`))
            (`MaterialInstanceDynamic.SetScalarParameterValue` _skyspherematerial_4 "CloudsMask02SmoothStepMin" (`self.CloudsMask02SmoothStepMin`))
            (`MaterialInstanceDynamic.SetScalarParameterValue` _skyspherematerial_4 "CloudsMask02SmoothStepRange" (`self.CloudsMask02SmoothStepRange`)))
          (:`then_3`
            (`MaterialInstanceDynamic.SetTextureParameterValue` _skyspherematerial_6 "StarsTexture" (`self.StarsTexture`))
            (`MaterialInstanceDynamic.SetScalarParameterValue` _skyspherematerial_6 "StarsIntensity" (`self.StarsIntensity`))
            (`MaterialInstanceDynamic.SetScalarParameterValue` _skyspherematerial_6 "StarsTilingU" (`self.StarsTilingU`))
            (`MaterialInstanceDynamic.SetScalarParameterValue` _skyspherematerial_6 "StarsTilingV" (`self.StarsTilingV`))
            (`MaterialInstanceDynamic.SetScalarParameterValue` _skyspherematerial_6 "LightSourceRadius" (`self.LightSourceRadius`))
            (if (and (`self.UseMainLight`) (`self.LightSourceLinkedToMainLight`))
              (set `self.LightSourceColor` (`self.MainLightColor`)))
            (`MaterialInstanceDynamic.SetVectorParameterValue` _skyspherematerial_6 "LightSourceColor" (`self.LightSourceColor`)))))
      (:`NewEnumerator3`
        (`MaterialInstanceDynamic.SetVectorParameterValue` _skyspherematerial_5 "BaseColor" (`self.BaseColor`))
        (if (`self.UseAmbientSkyLight`)
          (set `self.Cubemap` (`self.AmbientCubemap`)))
        (`MaterialInstanceDynamic.SetTextureParameterValue` _skyspherematerial_5 "Cubemap" (`self.Cubemap`))
        (goto _label)))
    (else
      (`ActorComponent.K2_DestroyComponent` (`self.SkySphere`)))))

(fn `UserConstructionScript`
  (`self.AmbientSkyLightInit`)
  (`self.DirectionalLightInit`)
  (`self.MaterialParameterCollectionInit`)
  (`self.ExponentialHeightFogInit`)
  (`self.AtmosphericFogInit`)
  (`self.SkySphereInit`))